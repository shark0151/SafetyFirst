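; Player character Blueprint with basic movement and a knockback reaction to being hit by an SUV.
; Axis inputs move it relative to the camera's forward and right vectors, turn controller yaw, and an action triggers jump.
; Capsule hits print the other actor's name; SUV_BP1 hits apply an impulse along the impact normal scaled by vehicle speed and mass.
; The X key fires that same impulse node directly, in a section marked garbage.
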(event `InputAxis|MoveForward`
  (params (AxisValue :type "Float (single-precision)"))
  (`PawnMovementComponent.AddInputVector` (`self.CharacterMovement`) (* (`KismetMathLibrary.GetForwardVector` (`SceneComponent.K2_GetComponentRotation` (`self.Camera`))) AxisValue) false))

(event `InputAxis|Turn`
  (params (AxisValue :type "Float (single-precision)"))
  (`self.AddControllerYawInput` AxisValue))

(event `InputAxis|MoveRight`
  (params (AxisValue :type "Float (single-precision)"))
  (`PawnMovementComponent.AddInputVector` (`self.CharacterMovement`) (* (`KismetMathLibrary.GetRightVector` (`SceneComponent.K2_GetComponentRotation` (`self.Camera`))) AxisValue) false))

(event `InputAction|Jump`
  (params (Key :type "Key Structure"))
  (:`Pressed`
    (`self.Jump`)))

(event `Key|X`
  (params (Key :type "Key Structure"))
  ;[1 1 1] garbage
  (:`Pressed`
    (`CharacterMovementComponent.AddImpulse` (`self.CharacterMovement`) (* (* (* (`.ImpactNormal` (`GameplayStatics.BreakHitResult` (stale `self.CapsuleComponent.OnComponentHit` Hit))) (`KismetMathLibrary.VSize` (`self.GetVelocity` (stale `self.CapsuleComponent.OnComponentHit` _assuv_bp1)))) (`PrimitiveComponent.GetMass` (`WheeledVehicle.Mesh` (stale `self.CapsuleComponent.OnComponentHit` _assuv_bp1)))) 1.0) false :!label _label)))

(event `self.CapsuleComponent.OnComponentHit`
  (params (HitComponent :type "PrimitiveComponent Object Reference") (OtherActor :type "Actor Object Reference") (OtherComp :type "PrimitiveComponent Object Reference") (NormalImpulse :type "Vector Structure") (Hit :type "HitResult Structure (by ref)"))
  ;[1 1 1] garbage
  (`KismetSystemLibrary.PrintString` (`KismetSystemLibrary.GetDisplayName` OtherActor))
  (bind _assuv_bp1 (cast `/Game/Car/SUV_BP1` (`.HitActor` (`GameplayStatics.BreakHitResult` Hit))))
  (goto _label))

(fn `UserConstructionScript`)