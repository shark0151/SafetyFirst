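; StopGameplay is an actor that judges whether the player comes to a stop inside a target zone.
; Each Tick it checks Player_BP actors overlapping Box1 and, when one is nearly stationary, calls Pass on NewPlayerController and latches its Pass flag.
; Any overlap ending on the separate Box component before that flag is set calls Failed on the controller, with no filter on the leaving actor.
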(event `self.ReceiveTick`
  (params (DeltaSeconds :type "Float (single-precision)"))
  (if (not (`self.Pass`))
    (for _array_element (`PrimitiveComponent.GetOverlappingActors` (`self.Box1`) "/Game/bike/Player_BP.Player_BP_C")
      (if (<= (`KismetMathLibrary.VSize` (`self.GetVelocity` _array_element)) 0.1)
        (bind _asnew_player_controller (cast `/Game/Blueprints/NewPlayerController` (`GameplayStatics.GetPlayerController` 0)))
        (`/Game/Blueprints/NewPlayerController.Pass` _asnew_player_controller)
        (set `self.Pass` true)))))

(event `self.Box.OnComponentEndOverlap`
  (params (OverlappedComponent :type "PrimitiveComponent Object Reference") (OtherActor :type "Actor Object Reference") (OtherComp :type "PrimitiveComponent Object Reference") (OtherBodyIndex :type Integer))
  (if (not (`self.Pass`))
    (bind _asnew_player_controller (cast `/Game/Blueprints/NewPlayerController` (`GameplayStatics.GetPlayerController` 0)))
    (`/Game/Blueprints/NewPlayerController.Failed` _asnew_player_controller)))

(fn `UserConstructionScript`)