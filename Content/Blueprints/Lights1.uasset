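; Traffic light actor that cycles green, yellow and red materials and reports stop states to vehicles.
; Tick advances a scaled timer through one of two offset phase sequences, selected by Alternate, by swapping lamp materials.
; For each SUV_BP overlapping the Box, it sets RedLight on yellow or red, then scans all actors to update every StopRedLight.
; DisableCollision turns off the Box at BeginPlay.
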(event `self.ReceiveBeginPlay`
  (if (`self.DisableCollision`)
    (`PrimitiveComponent.SetCollisionEnabled` (`self.Box`) "NoCollision")))

(event `self.ReceiveTick`
  (params (DeltaSeconds :type "Float (single-precision)"))
  (bind _returnvalue (or (== (`PrimitiveComponent.GetMaterial` (`self.Yellow`) 0) "/Game/Blueprints/YellowOn.YellowOn") (== (`PrimitiveComponent.GetMaterial` (`self.Red`) 0) "/Game/Blueprints/RedOn.RedOn")))
  (set `self.timer` (+ (`self.timer`) (* DeltaSeconds 0.7)))
  (`|ExecutionSequence`
    (:`then_0`
      (if (`self.Alternate`)
        (if (>= (`self.timer`) 5.0)
          (if (>= (`self.timer`) 7.0)
            (if (>= (`self.timer`) 16.0)
              (if (>= (`self.timer`) 18.0)
                (set `self.timer` 0.0)
                (else
                  (`PrimitiveComponent.SetMaterial` (`self.Green`) 0 "/Game/Blueprints/GreenOff.GreenOff")
                  (`PrimitiveComponent.SetMaterial` (`self.Yellow`) 0 "/Game/Blueprints/YellowOn.YellowOn")
                  (`PrimitiveComponent.SetMaterial` (`self.Red`) 0 "/Game/Blueprints/RedOff.RedOff")))
              (else
                (`PrimitiveComponent.SetMaterial` (`self.Green`) 0 "/Game/Blueprints/GreenOff.GreenOff")
                (`PrimitiveComponent.SetMaterial` (`self.Yellow`) 0 "/Game/Blueprints/YellowOff.YellowOff")
                (`PrimitiveComponent.SetMaterial` (`self.Red`) 0 "/Game/Blueprints/RedOn.RedOn")))
            (else
              (`PrimitiveComponent.SetMaterial` (`self.Green`) 0 "/Game/Blueprints/GreenOff.GreenOff")
              (`PrimitiveComponent.SetMaterial` (`self.Yellow`) 0 "/Game/Blueprints/YellowOn.YellowOn")
              (`PrimitiveComponent.SetMaterial` (`self.Red`) 0 "/Game/Blueprints/RedOff.RedOff")))
          (else
            (`PrimitiveComponent.SetMaterial` (`self.Green`) 0 "/Game/Blueprints/GreenOn.GreenOn")
            (`PrimitiveComponent.SetMaterial` (`self.Yellow`) 0 "/Game/Blueprints/YellowOff.YellowOff")
            (`PrimitiveComponent.SetMaterial` (`self.Red`) 0 "/Game/Blueprints/RedOff.RedOff")))
        (elif (>= (`self.timer`) 7.0)
          (if (>= (`self.timer`) 9.0)
            (if (>= (`self.timer`) 14.0)
              (if (>= (`self.timer`) 16.0)
                (if (>= (`self.timer`) 18.0)
                  (set `self.timer` 0.0)
                  (else
                    (`PrimitiveComponent.SetMaterial` (`self.Green`) 0 "/Game/Blueprints/GreenOff.GreenOff")
                    (`PrimitiveComponent.SetMaterial` (`self.Yellow`) 0 "/Game/Blueprints/YellowOff.YellowOff")
                    (`PrimitiveComponent.SetMaterial` (`self.Red`) 0 "/Game/Blueprints/RedOn.RedOn")))
                (else
                  (`PrimitiveComponent.SetMaterial` (`self.Green`) 0 "/Game/Blueprints/GreenOff.GreenOff")
                  (`PrimitiveComponent.SetMaterial` (`self.Yellow`) 0 "/Game/Blueprints/YellowOn.YellowOn")
                  (`PrimitiveComponent.SetMaterial` (`self.Red`) 0 "/Game/Blueprints/RedOff.RedOff")))
              (else
                (`PrimitiveComponent.SetMaterial` (`self.Green`) 0 "/Game/Blueprints/GreenOn.GreenOn")
                (`PrimitiveComponent.SetMaterial` (`self.Yellow`) 0 "/Game/Blueprints/YellowOff.YellowOff")
                (`PrimitiveComponent.SetMaterial` (`self.Red`) 0 "/Game/Blueprints/RedOff.RedOff")))
            (else
              (`PrimitiveComponent.SetMaterial` (`self.Green`) 0 "/Game/Blueprints/GreenOff.GreenOff")
              (`PrimitiveComponent.SetMaterial` (`self.Yellow`) 0 "/Game/Blueprints/YellowOn.YellowOn")
              (`PrimitiveComponent.SetMaterial` (`self.Red`) 0 "/Game/Blueprints/RedOff.RedOff")))
          (else
            (`PrimitiveComponent.SetMaterial` (`self.Green`) 0 "/Game/Blueprints/GreenOff.GreenOff")
            (`PrimitiveComponent.SetMaterial` (`self.Yellow`) 0 "/Game/Blueprints/YellowOff.YellowOff")
            (`PrimitiveComponent.SetMaterial` (`self.Red`) 0 "/Game/Blueprints/RedOn.RedOn")))))
    (:`then_1`
      (for _array_element (`PrimitiveComponent.GetOverlappingActors` (`self.Box`) null)
        (bind _assuv_bp (cast `/Game/Car/SUV_BP` _array_element))
        (set `/Game/Car/SUV_BP.RedLight` _returnvalue _assuv_bp)
        (bind _outactors (`GameplayStatics.GetAllActorsOfClass` "/Script/Engine.Actor"))
        (for _array_element_2 _outactors
          (bind _asstop_red_light (cast `/Game/Blueprints/StopRedLight` _array_element_2))
          (set `/Game/Blueprints/StopRedLight.IsRedLight` _returnvalue _asstop_red_light))))))

(fn `UserConstructionScript`)