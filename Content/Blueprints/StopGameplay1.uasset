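; StopGameplay1 is a trigger-volume actor that reports a pass or fail to NewPlayerController.
; Player_BP entering the BoEnd trigger calls Pass on the controller and sets the actor's Pass flag.
; Any actor leaving Box before that flag is set calls Failed, unless it still overlaps a StopGameplay1 actor, so overlapping volumes form one continuous allowed area.
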(event `self.ReceiveTick`
  (params (DeltaSeconds :type "Float (single-precision)")))

(event `self.Box.OnComponentEndOverlap`
  (params (OverlappedComponent :type "PrimitiveComponent Object Reference") (OtherActor :type "Actor Object Reference") (OtherComp :type "PrimitiveComponent Object Reference") (OtherBodyIndex :type Integer))
  (if (`self.Pass`)
    _
    (elif (not (> (`KismetArrayLibrary.Array_Length` (`self.GetOverlappingActors` OtherActor "StopGameplay1_C")) 0))
      (bind _asnew_player_controller (cast `/Game/Blueprints/NewPlayerController` (`GameplayStatics.GetPlayerController` 0)))
      (`/Game/Blueprints/NewPlayerController.Failed` _asnew_player_controller))))

(event `self.BoEnd.OnComponentBeginOverlap`
  (params (OverlappedComponent :type "PrimitiveComponent Object Reference") (OtherActor :type "Actor Object Reference") (OtherComp :type "PrimitiveComponent Object Reference") (OtherBodyIndex :type Integer) (bFromSweep :type Boolean) (SweepResult :type "HitResult Structure (by ref)"))
  (if (== (`GameplayStatics.GetObjectClass` OtherActor) "/Game/bike/Player_BP.Player_BP_C")
    (bind _asnew_player_controller (cast `/Game/Blueprints/NewPlayerController` (`GameplayStatics.GetPlayerController` 0)))
    (`/Game/Blueprints/NewPlayerController.Pass` _asnew_player_controller)
    (set `self.Pass` true)))

(fn `UserConstructionScript`)