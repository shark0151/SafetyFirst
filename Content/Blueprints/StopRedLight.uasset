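; StopRedLight is a Blueprint actor that fails the player for moving through its zone during a red light.
; Each tick, while IsRedLight is set, it checks Player_BP actors overlapping its Box.
; Any actor with velocity above a near-zero threshold triggers Failed on the NewPlayerController of player 0.
; The file itself never changes IsRedLight.
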(event `self.ReceiveTick`
  (params (DeltaSeconds :type "Float (single-precision)"))
  (if (`self.IsRedLight`)
    (for _array_element (`PrimitiveComponent.GetOverlappingActors` (`self.Box`) "/Game/bike/Player_BP.Player_BP_C")
      (if (not (<= (`KismetMathLibrary.VSize` (`self.GetVelocity` _array_element)) 0.1))
        (bind _asnew_player_controller (cast `/Game/Blueprints/NewPlayerController` (`GameplayStatics.GetPlayerController` 0)))
        (`/Game/Blueprints/NewPlayerController.Failed` _asnew_player_controller)))))

(fn `UserConstructionScript`)