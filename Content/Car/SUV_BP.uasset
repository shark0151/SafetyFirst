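; AI-driven SUV vehicle that follows the spline of the first Path actor in the level, with a randomized paint color.
; Each tick, GetPath advances the target spline point when near and derives steering from yaw error, easing throttle in turns.
; A forward sphere trace, shortened while steering, triggers braking and handbrake on obstacles.
; An externally set RedLight flag, cleared each tick, also brakes; both conditions light the brake reflector.
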(event `self.ReceiveTick`
  (params (DeltaSeconds :type "Float (single-precision)"))
  (bind _vehiclemovement (`self.VehicleMovement`))
  (bind _mesh (`self.Mesh`))
  (bind _returnvalue (+ (`self.K2_GetActorLocation`) (0.0 0.0 170.0)))
  (bind _outactors (`GameplayStatics.GetAllActorsOfClass` "/Game/Car/Path.Path_C"))
  (bind (_steering _throttle _breaking) (`self.GetPath` _outactors))
  (`WheeledVehicleMovementComponent.SetSteeringInput` _vehiclemovement _steering)
  (`WheeledVehicleMovementComponent.SetThrottleInput` _vehiclemovement _throttle)
  (`WheeledVehicleMovementComponent.SetBrakeInput` _vehiclemovement _breaking)
  (`WheeledVehicleMovementComponent.SetHandbrakeInput` _vehiclemovement (`self.Stop`))
  (bind (_outhit _returnvalue_2) (`KismetSystemLibrary.SphereTraceSingle` _returnvalue (+ (* (`SceneComponent.GetForwardVector` (`self.Mesh`)) (- 850.0 (* (`KismetMathLibrary.Abs` _steering) 500.0))) _returnvalue) 120.0 "TraceTypeQuery1"))
  (set `self.Stop` _returnvalue_2)
  (if (or (`self.RedLight`) (`self.Stop`))
    (`PrimitiveComponent.SetMaterial` _mesh 11 "/Game/DriveableCar_basic/Materials/Material_Instances/reflectors/MI_Reflector_RED_Emmisive.MI_Reflector_RED_Emmisive")
    (else
      (`PrimitiveComponent.SetMaterial` _mesh 11 "/Game/DriveableCar_basic/Materials/Material_Instances/reflectors/MI_Reflector_RED.MI_Reflector_RED")))
  (set `self.RedLight` false))

(event `InputAxis|MoveForward`
  (params (AxisValue :type "Float (single-precision)"))
  (`WheeledVehicleMovementComponent.SetThrottleInput` (`self.VehicleMovement`) AxisValue))

(event `InputAxis|Turn`
  (params (AxisValue :type "Float (single-precision)"))
  (`self.AddControllerYawInput` AxisValue))

(event `InputAxis|LookUp`
  (params (AxisValue :type "Float (single-precision)"))
  (`self.AddControllerPitchInput` AxisValue))

(event `InputAxis|MoveRight`
  (params (AxisValue :type "Float (single-precision)"))
  (`WheeledVehicleMovementComponent.SetSteeringInput` (`self.VehicleMovement`) AxisValue))

(event `self.ReceiveBeginPlay`
  (bind _outactors (`GameplayStatics.GetAllActorsOfClass` "/Game/Car/Path.Path_C"))
  (bind _returnvalue (`PrimitiveComponent.CreateDynamicMaterialInstance` (`self.Mesh`) 0 "/Game/DriveableCar_basic/Materials/Material_Instances/cars/carpaint/MI_CarPaint_06_WhitePearl.MI_CarPaint_06_WhitePearl" "None"))
  (`MaterialInstanceDynamic.SetVectorParameterValue` _returnvalue "Base Color" (`KismetMathLibrary.Conv_VectorToLinearColor` (`KismetMathLibrary.RandomPointInBoundingBox` (0.0 0.0 0.0) (0.8 0.7 0.8))))
  (bind _output (`|GetArrayItem` _outactors))
  (bind _output_get (set `self.Path Length` (`SplineComponent.GetNumberOfSplinePoints` (`/Game/Car/Path.Spline` _output))))
  (bind _returnvalue_2 (+ (`KismetMathLibrary.FTrunc` (`SplineComponent.FindInputKeyClosestToWorldLocation` (`/Game/Car/Path.Spline` _output) (`self.K2_GetActorLocation`))) 1))
  (if (< _returnvalue_2 _output_get)
    (set `self.PathIndex` _returnvalue_2)
    (else
      (set `self.PathIndex` 0))))

(fn `GetPath`
  (params (Path :type "Array of /Game/Car/Path Object Reference"))
  (returns (Steering :type "Float (double-precision)") (Throttle :type "Float (double-precision)") (Breaking :type "Float (double-precision)"))
  (bind _returnvalue (`self.K2_GetActorLocation`))
  (bind _returnvalue_2 (or (`self.RedLight`) (`self.Stop`)))
  (bind _returnvalue_3 (`SplineComponent.GetLocationAtSplinePoint` (`/Game/Car/Path.Spline` (`|GetArrayItem` Path)) (`self.PathIndex`) "World"))
  (bind (_returnvalue_roll _returnvalue_pitch _returnvalue_yaw) (`KismetMathLibrary.BreakRotator` (`KismetMathLibrary.NormalizedDeltaRotator` (`KismetMathLibrary.FindLookAtRotation` _returnvalue _returnvalue_3) (`self.K2_GetActorRotation`))))
  (bind _returnvalue_4 (`KismetMathLibrary.MapRangeClamped` _returnvalue_yaw -90.0 90.0 -1.0 1.0))
  (if (== _returnvalue_3 _returnvalue :`ErrorTolerance` 500.0)
    (if (< (`self.PathIndex`) (+ (`self.Path Length`) 1))
      (`/Engine/EditorBlueprintResources/StandardMacros.IncrementInt` (`self.PathIndex`)
        (:`  `
          _))
      (else
        (set `self.PathIndex` 0))))
  (return _returnvalue_4 (* (- 0.7 (* (`KismetMathLibrary.Abs` _returnvalue_4) 0.2)) (`KismetMathLibrary.Conv_BoolToDouble` (not _returnvalue_2))) (`KismetMathLibrary.Conv_BoolToDouble` _returnvalue_2)))

(fn `UserConstructionScript`)