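; Controller for the Xsolla demo's character panel that loads and saves the player's login attributes.
; Refresh requests editable and read-only attributes in parallel, using a map of ready flags to wait for both callbacks before filling and activating the panel.
; User details combine subsystem data, token parameters and a level read from a local save.
; Saving chains attribute modification into removal, with a loader shown meanwhile.
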(event `/XsollaLogin/Login/Controllers/BPI_CharacterController.RefreshCharacterPanel`
  (params (CharacterPanel :type "/XsollaLogin/Login/Interface/BPI_CharacterPanel Interface"))
  ;[1 1 1] Refresh character panel
  (`self.ResetAttributeRequestsFlags`)
  (`/XsollaLogin/Common/BP_DemoUtils.ShowLoader` true)
  (`XsollaLoginSubsystem.UpdateUserAttributes` :`self` (subsystem `XsollaLoginSubsystem`) :`AuthToken` (`/XsollaLogin/Login/Misc/BP_TokenUtils.GetToken`) :`SuccessCallback` (delegate `OnAttributesUpdateSuccess`) :`ErrorCallback` (`|CreateDelegate` :!event `ShowError`))
  (`XsollaLoginSubsystem.UpdateUserReadOnlyAttributes` :`self` (subsystem `XsollaLoginSubsystem`) :`AuthToken` (`/XsollaLogin/Login/Misc/BP_TokenUtils.GetToken`) :`SuccessCallback` (delegate `OnReadOnlyAttributesUpdateSuccess`) :`ErrorCallback` (`|CreateDelegate` :!event `ShowError`)))

(event `OnReadOnlyAttributesUpdateSuccess`
  ;[1 1 1] Refresh character panel
  (`BlueprintMapLibrary.Map_Add` (`self.AttributesReady`) "attributes_readonly_ready" true)
  (bind _ready (`self.AttributeRequestReady` :!label _label))
  (if _ready
    (`/XsollaLogin/Common/BP_DemoUtils.ShowLoader` false)
    (bind _returnvalue (`XsollaLoginSubsystem.GetUserAttributes` (subsystem `XsollaLoginSubsystem`)))
    (bind _attributesdata (`self.CreateAttributesData` _returnvalue (stale `/XsollaLogin/Login/Controllers/BPI_CharacterController.RefreshCharacterPanel` CharacterPanel)))
    (bind _returnvalue_2 (`XsollaLoginSubsystem.GetUserReadOnlyAttributes` (subsystem `XsollaLoginSubsystem`)))
    (bind _attributesdata_2 (`self.CreateAttributesData` _returnvalue_2 (stale `/XsollaLogin/Login/Controllers/BPI_CharacterController.RefreshCharacterPanel` CharacterPanel)))
    (bind _userdata (`self.CreateUserDetailsData`))
    (`/XsollaLogin/Login/Interface/BPI_CharacterPanel.RefreshCharacterData` (stale `/XsollaLogin/Login/Controllers/BPI_CharacterController.RefreshCharacterPanel` CharacterPanel) _attributesdata _attributesdata_2 _userdata)
    (`/XsollaLogin/Login/Interface/BPI_DemoWidget.ActivateCharacterPanel` (`self.DemoWidget`))))

(event `OnAttributesUpdateSuccess`
  ;[1 1 1] Refresh character panel
  (`BlueprintMapLibrary.Map_Add` (`self.AttributesReady`) "attributes_ready" true)
  (goto _label))

(event `/XsollaLogin/Login/Controllers/BPI_CharacterController.OnUserAttributesSaveInitiated`
  (params (AttributesSaveData :type "/XsollaLogin/Login/Data/BP_AttributeSaveData Object Reference"))
  ;[1 1 1] Save user attributes
  (bind _attributes (`self.ParseAttributesData` (`/XsollaLogin/Login/Data/BP_AttributeSaveData.AttributesToModify` AttributesSaveData)))
  (`/XsollaLogin/Common/BP_DemoUtils.ShowLoader` true)
  (`XsollaLoginSubsystem.ModifyUserAttributes` (subsystem `XsollaLoginSubsystem`) (`/XsollaLogin/Login/Misc/BP_TokenUtils.GetToken`) _attributes (delegate `OnModifyAttributesSuccess`) (`|CreateDelegate` :!event `ShowError`)))

(event `OnModifyAttributesSuccess`
  ;[1 1 1] Save user attributes
  (`XsollaLoginSubsystem.RemoveUserAttributes` (subsystem `XsollaLoginSubsystem`) (`/XsollaLogin/Login/Misc/BP_TokenUtils.GetToken`) (`/XsollaLogin/Login/Data/BP_AttributeSaveData.AttributesToRemove` (stale `/XsollaLogin/Login/Controllers/BPI_CharacterController.OnUserAttributesSaveInitiated` AttributesSaveData)) (delegate `OnRemoveAttributesSuccess`) (`|CreateDelegate` :!event `ShowError`)))

(event `OnRemoveAttributesSuccess`
  ;[1 1 1] Save user attributes
  (`/XsollaLogin/Common/BP_DemoUtils.ShowLoader` false))

(fn `AttributeRequestReady`
  (returns (Ready :type Boolean))
  (bind _keys (`BlueprintMapLibrary.Map_Keys` (`self.AttributesReady`)))
  (for _array_element _keys
    (if (not (`BlueprintMapLibrary.Map_Find` (`self.AttributesReady`) _array_element))
      (return false)))
  (return true))

(fn `CreateAttributesData`
  (params (Attributes :type "Array of XsollaUserAttribute Structure (by ref)") (Profile :type "/XsollaLogin/Login/Interface/BPI_CharacterPanel Interface"))
  (returns (AttributesData :type "Array of /XsollaLogin/Login/Data/BP_AttributeItemData Object Reference"))
  (locals (AttributeItemData :type "Array of /XsollaLogin/Login/Data/BP_AttributeItemData Object Reference"))
  (for _array_element Attributes
    (bind (_key _permission _value) (break `XsollaUserAttribute` _array_element))
    (bind _returnvalue (`|GenericCreateObject` "/XsollaLogin/Login/Data/BP_AttributeItemData.BP_AttributeItemData_C" self _key _permission _value Profile))
    (`KismetArrayLibrary.Array_Add` (`local.AttributeItemData`) _returnvalue))
  (return (`local.AttributeItemData`)))

(fn `CreateUserDetailsData`
  (returns (UserData :type "/XsollaLogin/Login/Interface/BPI_UserDetailsData Interface"))
  (bind _returnvalue (`|GenericCreateObject` "/XsollaLogin/Login/Data/BP_UserDetailsData.BP_UserDetailsData_C" self (`XsollaLoginSubsystem.GetUserDetails` (subsystem `XsollaLoginSubsystem`)) (`self.GetCurrentUserLevel`) (`/XsollaLogin/Login/Misc/BP_TokenUtils.GetTokenParameter` "username") (`KismetStringLibrary.EqualEqual_StrStr` (`/XsollaLogin/Login/Misc/BP_TokenUtils.GetTokenParameter` "type") "xsolla_login")))
  (bind _iconsloader (`/XsollaLogin/Login/Interface/BPI_Demo.GetIconsLoader` (`self.Demo`)))
  (`/XsollaLogin/Login/Interface/BPI_IconsLoader.LoadIcons` _iconsloader (`|MakeArray` _returnvalue :!type "/XsollaLogin/Common/Interface/BPI_IconPresenter Interface"))
  (return _returnvalue))

(fn `GetCurrentUserLevel`
  (returns (Value :type Integer))
  (bind _returnvalue (`GameplayStatics.LoadGameFromSlot` "UserLevelData"))
  (bind _asbp_user_level_save_data (cast `/XsollaLogin/Login/Data/BP_UserLevelSaveData` _returnvalue)
    (:`then`
      (bind (_value _returnvalue_2) (`BlueprintMapLibrary.Map_Find` (`/XsollaLogin/Login/Data/BP_UserLevelSaveData.UserLevels` _asbp_user_level_save_data) (`/XsollaLogin/Login/Misc/BP_TokenUtils.GetTokenParameter` "sub")))
      (if _returnvalue_2
        (return _value)
        (else
          (return 1))))
    (:`CastFailed`
      (return 1))))

(fn `Init`
  (params (InDemo :type "/XsollaLogin/Login/Interface/BPI_Demo Interface") (InDemoWidget :type "/XsollaLogin/Login/Interface/BPI_DemoWidget Interface"))
  (set `self.Demo` InDemo)
  (set `self.DemoWidget` InDemoWidget))

(fn `ParseAttributesData`
  (params (AttributesData :type "Array of /XsollaLogin/Login/Data/BP_AttributeItemData Object Reference (by ref)"))
  (returns (Attributes :type "Array of XsollaUserAttribute Structure"))
  (locals (XsollaAttributes :type "Array of XsollaUserAttribute Structure"))
  (for _array_element AttributesData
    (`KismetArrayLibrary.Array_Add` (`local.XsollaAttributes`) (make `XsollaUserAttribute` (`/XsollaLogin/Login/Data/BP_AttributeItemData.Key` _array_element) (`/XsollaLogin/Login/Data/BP_AttributeItemData.Permission` _array_element) (`/XsollaLogin/Login/Data/BP_AttributeItemData.Value` _array_element))))
  (return (`local.XsollaAttributes`)))

(fn `ResetAttributeRequestsFlags`
  (bind _attributesready (`self.AttributesReady`))
  (`BlueprintMapLibrary.Map_Clear` _attributesready)
  (`BlueprintMapLibrary.Map_Add` _attributesready "attributes_ready")
  (`BlueprintMapLibrary.Map_Add` _attributesready "attributes_readonly_ready"))

(fn `ShowError`
  (params (Code :type String) (Description :type String))
  (`/XsollaLogin/Common/BP_DemoUtils.ShowLoginError` Code Description))